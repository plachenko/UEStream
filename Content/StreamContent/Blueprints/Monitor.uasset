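; Monitor is an actor that shows a live Spout video feed on its mesh and returns to its start transform after landing on the landscape.
; The construction script sets the mesh and creates a dynamic material, whose texture parameter Tick updates from the named Spout receiver.
; Hits from ThrowObj activate that object's particles, while Landscape hits trigger a guarded, delayed reset.
; EndPlay calls CloseSender with the Spout name.
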(event `self.ReceiveBeginPlay`
  (set `self.StartTransform` (`self.GetTransform`)))

(event `ResetTransform`
  ;[1 1 1] reset position
  (`SceneComponent.K2_SetWorldTransform` (`self.StaticMesh`) (`self.StartTransform`) false false))

(event `self.ReceiveHit`
  (params (MyComp :type "PrimitiveComponent Object Reference") (Other :type "Actor Object Reference") (OtherComp :type "PrimitiveComponent Object Reference") (bSelfMoved :type Boolean) (HitLocation :type "Vector Structure") (HitNormal :type "Vector Structure") (NormalImpulse :type "Vector Structure") (Hit :type "HitResult Structure (by ref)"))
  ;[1 1 1] on hit
  (bind _asthrow_obj (cast `/Game/StreamContent/Blueprints/ThrowObj` Other)
    (:`then`
      (`ActorComponent.Activate` (`/Game/StreamContent/Blueprints/ThrowObj.ParticleSystem` _asthrow_obj) false))
    (:`CastFailed`
      (cast `Landscape` Other)
      (if (not (`self.HasHitFloor`))
        (set `self.HasHitFloor` true)
        (`KismetSystemLibrary.Delay` 1.0)
        (`self.ResetTransform`)
        (set `self.HasHitFloor` false)))))

(event `self.ReceiveTick`
  (params (DeltaSeconds :type "Float (single-precision)"))
  ;[1 1 1] set material
  (bind (_mat _texture) (`SpoutBPFunctionLibrary.SpoutReceiver` (`self.Spout Name`)))
  (`MaterialInstanceDynamic.SetTextureParameterValue` (`self.MonitorMat`) "Param" _texture)
  (`PrimitiveComponent.SetMaterial` (`self.StaticMesh`) 0 (`self.MonitorMat`)))

(event `self.ReceiveEndPlay`
  (params (EndPlayReason :type "EEndPlayReason Enum" :default "Destroyed"))
  (`SpoutBPFunctionLibrary.CloseSender` (`self.Spout Name`)))

(fn `UserConstructionScript`
  (`StaticMeshComponent.SetStaticMesh` (`self.StaticMesh`) (`self.MonitorMesh`))
  (bind _returnvalue (`KismetMaterialLibrary.CreateDynamicMaterialInstance` (`|GetArrayItem` (`MeshComponent.GetMaterials` (`self.StaticMesh`)))))
  (set `self.MonitorMat` _returnvalue))